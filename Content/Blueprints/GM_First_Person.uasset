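; First-person game mode that tracks connected players and provides player spawning.
; Login and logout add or remove PC_FirstPerson controllers from an array, then tell GS_FirstPerson to update its player list after a short delay.
; SpawnPlayer, not called within this Blueprint, replaces a controller's pawn with a new possessed BP_FirstPersonCharacter at a random PlayerStart, falling back to just above the origin if none exist.
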(event `self.ReceiveBeginPlay`)

(event `self.K2_PostLogin`
  (params (NewPlayer :type "PlayerController Object Reference"))
  (bind _aspc_first_person (cast `/Game/Blueprints/PC_FirstPerson` NewPlayer))
  (`KismetArrayLibrary.Array_Add` (`self.PlayerControllers`) _aspc_first_person)
  (`KismetSystemLibrary.PrintString` (`KismetStringLibrary.Concat_StrStr` "Player Count: " (`KismetStringLibrary.Conv_IntToString` (`KismetArrayLibrary.Array_Length` (`self.PlayerControllers`)))))
  (`self.UpdatePlayerList` :!label _label))

(event `self.K2_OnLogout`
  (params (ExitingController :type "Controller Object Reference"))
  (bind _aspc_first_person (cast `/Game/Blueprints/PC_FirstPerson` ExitingController))
  (`KismetArrayLibrary.Array_RemoveItem` (`self.PlayerControllers`) _aspc_first_person)
  (goto _label))

(event `UpdatePlayerList`
  (`KismetSystemLibrary.Delay` 0.5)
  (bind _asgs_first_person (cast `/Game/Blueprints/GS_FirstPerson` (`GameplayStatics.GetGameState`)))
  (`/Game/Blueprints/GS_FirstPerson.UpdatePlayerList` _asgs_first_person)
  (`KismetSystemLibrary.PrintString` "GM_FirstPerson"))

(fn `FindRandomPlayerStart`
  (returns (Transform :type "Transform Structure"))
  (bind _outactors (`GameplayStatics.GetAllActorsOfClass` "/Script/Engine.PlayerStart"))
  (bind _returnvalue (`KismetArrayLibrary.Array_Length` _outactors))
  (if (== _returnvalue 0)
    (return (`KismetMathLibrary.MakeTransform` (0.0 0.0 100.0)))
    (else
      (return (`self.GetTransform` (`|GetArrayItem` _outactors (`KismetMathLibrary.RandomIntegerInRange` 0 (- _returnvalue 1))))))))

(fn `SpawnPlayer`
  (params (`Player Controller` :type "PlayerController Object Reference"))
  (bind _returnvalue (`Controller.K2_GetPawn` `Player Controller`))
  (`/Engine/EditorBlueprintResources/StandardMacros.IsValid` _returnvalue
    (:`Is Valid`
      (`self.K2_DestroyActor` _returnvalue))
    (:`Is Not Valid`
      _))
  (bind _returnvalue_2 (`|SpawnActorFromClass` "/Game/FirstPerson/Blueprints/BP_FirstPersonCharacter.BP_FirstPersonCharacter_C" (`self.FindRandomPlayerStart`) "Undefined" "MultiplyWithRoot" null null))
  (`Controller.Possess` (`local.Player Controller`) _returnvalue_2))

(fn `UserConstructionScript`)