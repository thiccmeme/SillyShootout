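; Base weapon actor that the first-person character picks up on overlap, then fires and scopes using values from WeaponStats.
; SpawnProjectile checks ammo, spawns projectiles along the camera rotation with random spread, passes them damage, speed and explosive settings, then gates refire with a delay.
; ActivateScope toggles camera zoom through an FOV offset.
; GetProjectileImage reads the projectile's image by briefly spawning one far above the weapon and destroying it.
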(event `GetProjectileImage`
  (bind _returnvalue (`|SpawnActorFromClass` (`self.ProjectileToSpawn`) (`KismetMathLibrary.Conv_VectorToTransform` (- (.location (`self.GetTransform`)) (0.0 0.0 -100000.0))) "Undefined" "MultiplyWithRoot" null 0.0 null 0 false null))
  (set `self.ProjectileImage` (`/Game/Blueprints/Weapons/Projectiles/BP_BaseProjectile.ProjectileImage` _returnvalue))
  (`self.K2_DestroyActor` _returnvalue))

(event `SpawnProjectile`
  (params (`Source Player` :type "/Game/FirstPerson/Blueprints/BP_FirstPersonCharacter Object Reference"))
  (bind _weaponstats (`self.WeaponStats`))
  (bind _hasammo (`/Game/Blueprints/Weapons/BP_WeaponStats.HasEnoughAmmo` (`self.WeaponStats`)))
  (if (and _hasammo (`self.CanSpawnProjectile`))
    (for _ (range 1 (+ (`/Game/Blueprints/Weapons/BP_WeaponStats.ProjectilesPerTrigger` (`self.WeaponStats`)) 1))
      (`|SpawnActorFromClass` (`self.ProjectileToSpawn`) (`self.CalculateSpawnTransform`) "AlwaysSpawn" "MultiplyWithRoot" (`self.PlayerRef`) (`/Game/Blueprints/Weapons/BP_WeaponStats.ProjectileSpeed` _weaponstats) null (`/Game/Blueprints/Weapons/BP_WeaponStats.Damage` _weaponstats) (`/Game/Blueprints/Weapons/BP_WeaponStats.IsProjectileExplosive` _weaponstats) null))
    (set `self.CanSpawnProjectile` false)
    (`KismetSystemLibrary.Delay` (`/Game/Blueprints/Weapons/BP_WeaponStats.FireRate` (`self.WeaponStats`)))
    (set `self.CanSpawnProjectile` true)))

(event `self.PlayerDetect.OnComponentBeginOverlap`
  (params (OverlappedComponent :type "PrimitiveComponent Object Reference") (OtherActor :type "Actor Object Reference") (OtherComp :type "PrimitiveComponent Object Reference") (OtherBodyIndex :type Integer) (bFromSweep :type Boolean) (SweepResult :type "HitResult Structure (by ref)"))
  (bind _asbp_first_person_character (cast `/Game/FirstPerson/Blueprints/BP_FirstPersonCharacter` OtherActor))
  (bind _output_get (set `self.PlayerRef` _asbp_first_person_character))
  (`/Engine/EditorBlueprintResources/StandardMacros.IsValid` _output_get
    (:`Is Valid`
      (`|ExecutionSequence`
        (:`then_0`
          (`/Game/FirstPerson/Blueprints/BP_FirstPersonCharacter.PickupWeapon` (`self.PlayerRef`) self))
        (:`then_1`
          (`self.SetOwner` (`self.PlayerRef`)))
        (:`then_2`
          (`PrimitiveComponent.SetCollisionEnabled` (`self.PlayerDetect`) "NoCollision")
          (`GameplayStatics.PlaySound2D` "/Game/Audio/FreeSoundPack/wav/Coin_Bag_3-1.Coin_Bag_3-1" 1.0 1.0 0.0 null null))))))

(fn `ActivateScope`
  (returns (InScopeMode :type Boolean))
  (bind _scopecameraoffset (`/Game/Blueprints/Weapons/BP_WeaponStats.ScopeCameraOffset` (`self.WeaponStats`)))
  (if (!= (`/Game/Blueprints/Weapons/BP_WeaponStats.ScopeCameraOffset` (`self.WeaponStats`)) 0.0)
    (set `CameraComponent.FieldOfView` (+ (`CameraComponent.FieldOfView` (`RPCTestCharacter.FirstPersonCameraComponent` (`self.PlayerRef`))) (`KismetMathLibrary.SelectFloat` (* _scopecameraoffset -1.0) _scopecameraoffset (`self.InScopeMode`))) (`RPCTestCharacter.FirstPersonCameraComponent` (`self.PlayerRef`)))
    (bind _output_get (set `self.InScopeMode` (not (`self.InScopeMode`))))
    (return _output_get)
    (else
      (return false))))

(fn `CalculateSpawnTransform`
  (returns (Transform :type "Transform Structure"))
  (bind _returnvalue (`SceneComponent.K2_GetComponentRotation` (`RPCTestCharacter.FirstPersonCameraComponent` (`self.PlayerRef`))))
  (return (`KismetMathLibrary.MakeTransform` (+ (`SceneComponent.K2_GetComponentLocation` (`self.Arrow`)) _returnvalue) (`KismetMathLibrary.MakeRotator` (.roll _returnvalue) (+ (.pitch _returnvalue) (`KismetMathLibrary.RandomFloatInRange` (`self.MinSpread`) (`self.MaxSpread`))) (+ (.yaw _returnvalue) (`KismetMathLibrary.RandomFloatInRange` (`self.MinSpread`) (`self.MaxSpread`)))))))

(fn `UserConstructionScript`)