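; Base projectile actor that damages first-person characters it overlaps and expires after a set lifetime.
; BeginPlay starts the lifetime timer, copies DamageAmount into the BPProjectileStats struct and plays a 2D spawn sound.
; Sphere overlaps ignore the owner, check IDamageable, then cast to BP_FirstPersonCharacter before sending damage and destroying the projectile.
; Sphere hits against object type "0" destroy it if DestroySelfOnHit is set; speed setters in the construction script are unconnected.
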(event `self.ReceiveBeginPlay`
  (`|ExecutionSequence`
    (:`then_1`
      (`KismetSystemLibrary.Delay` (`/Game/Blueprints/Weapons/Projectiles/BP_ProjectileStats.Duration` (`self.BP_ProjectileStats`)))
      (`self.K2_DestroyActor`))
    (:`then_2`
      (set `/Game/Blueprints/Weapons/Projectiles/BP_ProjectileStats.Damage` (`self.DamageAmount`) (`self.BP_ProjectileStats`)))
    (:`then_3`
      (`GameplayStatics.PlaySound2D` (`self.SoundOnSpawn`) 1.0 1.0 0.0 null null))))

(event `self.Sphere.OnComponentBeginOverlap`
  (params (OverlappedComponent :type "PrimitiveComponent Object Reference") (OtherActor :type "Actor Object Reference") (OtherComp :type "PrimitiveComponent Object Reference") (OtherBodyIndex :type Integer) (bFromSweep :type Boolean) (SweepResult :type "HitResult Structure (by ref)"))
  (if (!= OtherActor (`self.GetOwner`))
    (bind _output_get (set `self.HitActor` OtherActor))
    (if (`KismetSystemLibrary.DoesImplementInterface` _output_get "/Game/Blueprints/IDamageable.IDamageable_C")
      (bind _asbp_first_person_character (cast `/Game/FirstPerson/Blueprints/BP_FirstPersonCharacter` (`self.HitActor`)))
      (message `/Game/Blueprints/IDamageable.TakeDamage` _asbp_first_person_character (`/Game/Blueprints/Weapons/Projectiles/BP_ProjectileStats.Damage` (`self.BP_ProjectileStats`)))
      (`self.K2_DestroyActor`))))

(event `self.Sphere.OnComponentHit`
  (params (HitComponent :type "PrimitiveComponent Object Reference") (OtherActor :type "Actor Object Reference") (OtherComp :type "PrimitiveComponent Object Reference") (NormalImpulse :type "Vector Structure") (Hit :type "HitResult Structure (by ref)"))
  (if (`KismetStringLibrary.EqualEqual_StrStr` (`KismetStringLibrary.Conv_ByteToString` (`PrimitiveComponent.GetCollisionObjectType` OtherComp)) "0")
    (if (`/Game/Blueprints/Weapons/Projectiles/BP_ProjectileStats.Destroy Self On Hit` (`self.BP_ProjectileStats`))
      (`self.K2_DestroyActor`))))

(fn `UserConstructionScript`)