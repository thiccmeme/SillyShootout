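; BP_Explosive is an explosion damage actor in the weapon projectiles folder that hurts what its Sphere overlaps.
; On overlap with an IDamageable actor, it applies Damage through the interface, disables sphere collision, prints the target's name and destroys itself after a short delay.
; Non-damageable overlaps are ignored, leaving it in place.
; Unconnected leftover nodes hold an older character-specific damage path that never runs.
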(event `self.Sphere.OnComponentBeginOverlap`
  (params (OverlappedComponent :type "PrimitiveComponent Object Reference") (OtherActor :type "Actor Object Reference") (OtherComp :type "PrimitiveComponent Object Reference") (OtherBodyIndex :type Integer) (bFromSweep :type Boolean) (SweepResult :type "HitResult Structure (by ref)"))
  (bind _asidamageable (cast `/Game/Blueprints/IDamageable` OtherActor))
  (`/Game/Blueprints/IDamageable.TakeDamage` _asidamageable (`self.Damage`))
  (`PrimitiveComponent.SetCollisionEnabled` (`self.Sphere`) "NoCollision")
  (`KismetSystemLibrary.PrintString` (`KismetSystemLibrary.GetDisplayName` OtherActor))
  (`KismetSystemLibrary.Delay` 0.2)
  (`self.K2_DestroyActor`))

(fn `UserConstructionScript`)