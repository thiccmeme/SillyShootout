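; BP_FlameThrower is a flamethrower weapon Blueprint that so far contains only a hit-detection trace.
; Its SpawnProjectile event runs a sphere trace on the Visibility channel from the Arrow component to the FlameEnd component, standing in for a spawned projectile.
; The trace draws timed debug shapes, and its result is unused, so this graph applies no damage or effects.
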(event `self.SpawnProjectile`
  (params (`Source Player` :type "/Game/FirstPerson/Blueprints/BP_FirstPersonCharacter Object Reference"))
  (`KismetSystemLibrary.SphereTraceSingle` :`Start` (`SceneComponent.K2_GetComponentLocation` (`self.Arrow`)) :`End` (`SceneComponent.K2_GetComponentLocation` (`self.FlameEnd`)) :`Radius` 50.0 :`TraceChannel` "TraceTypeQuery1" :`DrawDebugType` "ForDuration"))

(fn `UserConstructionScript`
  (`parent.UserConstructionScript`))