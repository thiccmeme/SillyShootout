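; Base weapon actor that the first-person character picks up on overlap and that fires projectiles.
; PlayerDetect overlap stores the player, calls its PickupWeapon, sets ownership, disables detection collision and plays a sound.
; SpawnProjectile checks WeaponStats ammo, then spawns a projectile from the Arrow position plus camera rotation, aimed along the camera, passing speed and damage.
; A flag and Delay throttle fire rate; Shootall is an empty stub.
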(event `SpawnProjectile`
  (params (`Source Player` :type "/Game/FirstPerson/Blueprints/BP_FirstPersonCharacter Object Reference"))
  (bind _returnvalue (`SceneComponent.K2_GetComponentRotation` (`RPCTestCharacter.FirstPersonCameraComponent` (`self.PlayerRef`))))
  (bind _hasammo (`/Game/Blueprints/WeaponStats.HasEnoughAmmo` (`self.WeaponStats`)))
  (if (and _hasammo (`self.CanSpawnProjectile`))
    (`|SpawnActorFromClass` (`self.ProjectileToSpawn`) (`KismetMathLibrary.MakeTransform` (+ (`SceneComponent.K2_GetComponentLocation` (`self.Arrow`)) _returnvalue) _returnvalue) "AlwaysSpawn" "MultiplyWithRoot" (`self.PlayerRef`) (`/Game/Blueprints/WeaponStats.ProjectileSpeed` (`self.WeaponStats`)) null (`/Game/Blueprints/WeaponStats.Damage` (`self.WeaponStats`)) null)
    (set `self.CanSpawnProjectile` false)
    (`KismetSystemLibrary.Delay` (`/Game/Blueprints/WeaponStats.FireRate` (`self.WeaponStats`)))
    (set `self.CanSpawnProjectile` true)))

(event `self.PlayerDetect.OnComponentBeginOverlap`
  (params (OverlappedComponent :type "PrimitiveComponent Object Reference") (OtherActor :type "Actor Object Reference") (OtherComp :type "PrimitiveComponent Object Reference") (OtherBodyIndex :type Integer) (bFromSweep :type Boolean) (SweepResult :type "HitResult Structure (by ref)"))
  (bind _asbp_first_person_character (cast `/Game/FirstPerson/Blueprints/BP_FirstPersonCharacter` OtherActor))
  (bind _output_get (set `self.PlayerRef` _asbp_first_person_character))
  (`/Engine/EditorBlueprintResources/StandardMacros.IsValid` _output_get
    (:`Is Valid`
      (`|ExecutionSequence`
        (:`then_0`
          (`/Game/FirstPerson/Blueprints/BP_FirstPersonCharacter.PickupWeapon` (`self.PlayerRef`) self))
        (:`then_1`
          (`self.SetOwner` (`self.PlayerRef`)))
        (:`then_2`
          (`PrimitiveComponent.SetCollisionEnabled` (`self.PlayerDetect`) "NoCollision")
          (`GameplayStatics.PlaySound2D` "/Game/Audio/FreeSoundPack/wav/Coin_Bag_3-1.Coin_Bag_3-1" 1.0 1.0 0.0 null null))))))

(fn `Shootall`)

(fn `UserConstructionScript`)