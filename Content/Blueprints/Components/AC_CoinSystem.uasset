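; AC_CoinSystem is a component that tracks a coin count and ends the game when the count reaches its maximum.
; Increase and decrease events adjust the value, clamped between min and max, and print the new total on screen.
; Hitting the max on an increase triggers WinGame, which prints an end message, waits briefly, then asks the Gi_Adv_Fri game instance to open a level by name.
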(event `IncreaseCoinValue`
  (params (Value :type Integer))
  (`self.IncreaseValue` Value)
  (`KismetSystemLibrary.PrintString` (`KismetStringLibrary.Concat_StrStr` "Coins:" (`KismetStringLibrary.Conv_IntToString` (`self.CurrentValue`)))))

(event `DecreaseCoinValue`
  (params (Value :type Integer))
  (`self.DecreaseValue` Value)
  (`KismetSystemLibrary.PrintString` (`KismetStringLibrary.Concat_StrStr` "Coins:" (`KismetStringLibrary.Conv_IntToString` (`self.CurrentValue`)))))

(event `WinGame`
  (bind _asgi_adv_fri (cast `/Game/Blueprints/Gi_Adv_Fri` (`GameplayStatics.GetGameInstance`)))
  (`KismetSystemLibrary.PrintString` "END GAME")
  (`KismetSystemLibrary.Delay` 0.2)
  (`/Game/Blueprints/Gi_Adv_Fri.OpenLevel` _asgi_adv_fri))

(fn `DecreaseValue`
  (params (Value :type Integer))
  (set `self.CurrentValue` (`KismetMathLibrary.Clamp` (- (`self.CurrentValue`) Value) (`self.MinValue`) (`self.MaxValue`))))

(fn `IncreaseValue`
  (params (Value :type Integer))
  (bind _output_get (set `self.CurrentValue` (`KismetMathLibrary.Clamp` (+ (`self.CurrentValue`) Value) (`self.MinValue`) (`self.MaxValue`))))
  (if (>= _output_get (`self.MaxValue`))
    (`self.WinGame`)))