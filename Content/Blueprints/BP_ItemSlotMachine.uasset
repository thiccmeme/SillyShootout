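; BP_ItemSlotMachine is an item slot machine actor that spawns a random item and shows its image.
; Spawn picks a class from Items into SetItem, then calls ClientSideLogic to spawn it at the Plane's transform.
; That event passes the spawned item's image to the WBP_WeaponSlotMachine widget, then calls DelayEvent, whose body is not shown.
; SetItem has a RepNotify, but its handler is empty.
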(event `self.Spawn`
  (set `self.SetItem` (`KismetArrayLibrary.Array_Random` (`self.Items`)))
  (`self.ClientSideLogic`))

(event `self.ClientSideLogic`
  (bind _returnvalue (`|SpawnActorFromClass` (`self.SetItem`) (`SceneComponent.K2_GetComponentToWorld` (`self.Plane`)) "Undefined" "MultiplyWithRoot" null null))
  (bind _output_get (set `self.CurrentImage` (`/Game/Blueprints/Collectables/BP_BaseCollectable.ItemImage` _returnvalue)))
  (bind _aswbp_weapon_slot_machine (cast `/Game/Blueprints/WBP_WeaponSlotMachine` (`WidgetComponent.GetWidget` (`self.Widget`))))
  (`/Game/Blueprints/WBP_WeaponSlotMachine.SetWeaponImage` _aswbp_weapon_slot_machine _output_get)
  (`self.DelayEvent`))

(fn `OnRep_SetItem`)

(fn `UserConstructionScript`
  (`parent.UserConstructionScript`))