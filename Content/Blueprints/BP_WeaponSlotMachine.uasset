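; BP_WeaponSlotMachine is a coin-operated slot machine that spawns a random weapon with a random projectile type.
; When a first-person character with enough coins overlaps its box, it deducts coins, animates the lever and spawns the weapon at the plane.
; The widget shows both images, and a five-second lockout follows.
; The ammo multiplier is only printed, and that debug message re-rolls its values independently of the spawned result.
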(event `self.ReceiveBeginPlay`
  (bind _aswbp_weapon_slot_machine (cast `/Game/Blueprints/WBP_WeaponSlotMachine` (`WidgetComponent.GetWidget` (`self.Widget`))))
  (set `self.WeaponSlotMachineWBP` _aswbp_weapon_slot_machine))

(event `SpawnGun`)

(event `SetAmmo`
  (bind _outitem (`KismetArrayLibrary.Array_Random` (`self.Projectiles`)))
  (set `/Game/Blueprints/Weapons/BP_BaseWeapon.ProjectileToSpawn` _outitem (stale `self.Box.OnComponentBeginOverlap` _returnvalue))
  (`KismetSystemLibrary.PrintString` (`KismetStringLibrary.Concat_StrStr` " \nWeapon:" (`KismetSystemLibrary.GetClassDisplayName` (`KismetArrayLibrary.Array_Random` (`self.Weapons`))) " \nProjectile:" (`KismetSystemLibrary.GetClassDisplayName` _outitem) " \nAmmoMultiplier:" (`KismetStringLibrary.Conv_DoubleToString` (`KismetMathLibrary.RandomFloatInRange` (`self.MinAmmoMultiplier`) (`self.MaxAmmoMultiplier`)))))
  (`self.DelayEvent`))

(event `self.Box.OnComponentBeginOverlap`
  (params (OverlappedComponent :type "PrimitiveComponent Object Reference") (OtherActor :type "Actor Object Reference") (OtherComp :type "PrimitiveComponent Object Reference") (OtherBodyIndex :type Integer) (bFromSweep :type Boolean) (SweepResult :type "HitResult Structure (by ref)"))
  (bind _asbp_first_person_character (cast `/Game/FirstPerson/Blueprints/BP_FirstPersonCharacter` OtherActor))
  (if (`self.CurrentlyUsing`)
    _
    (elif (>= (`/Game/FirstPerson/Blueprints/BP_FirstPersonCharacter.CurrentCoins` _asbp_first_person_character) (`self.CoinValue`))
      (`self.RotateLever`)
      (`self.SpawnGun`)
      (`/Game/FirstPerson/Blueprints/BP_FirstPersonCharacter.DecCoins` _asbp_first_person_character (`self.CoinValue`))
      (`/Game/FirstPerson/Blueprints/BP_FirstPersonCharacter.UpdateGameHUD` _asbp_first_person_character)
      (set `self.CurrentlyUsing` true)
      (bind _returnvalue (`|SpawnActorFromClass` (`KismetArrayLibrary.Array_Random` (`self.Weapons`)) (`SceneComponent.K2_GetComponentToWorld` (`self.Plane`)) "AlwaysSpawn" "MultiplyWithRoot" null null))
      (`/Game/Blueprints/WBP_WeaponSlotMachine.SetWeaponImage` (`self.WeaponSlotMachineWBP`) (`/Game/Blueprints/Weapons/BP_BaseWeapon.WeaponImage` _returnvalue))
      (`self.SetAmmo`)
      (`/Game/Blueprints/Weapons/BP_BaseWeapon.GetProjectileImage` _returnvalue)
      (`/Game/Blueprints/WBP_WeaponSlotMachine.SetProjectileImage` (`self.WeaponSlotMachineWBP`) (`/Game/Blueprints/Weapons/BP_BaseWeapon.ProjectileImage` _returnvalue))
      (else
        (`KismetSystemLibrary.PrintString` "Not enough coin value")))))

(event `DelayEvent`
  (`KismetSystemLibrary.Delay` 5.0)
  (set `self.CurrentlyUsing` false))

(event `RotateLever`
  (bind (_direction _leverxrotation) (`Timeline|LeverTimeline2` :!via `PlayFromStart`)
    (:`Update`
      (`SceneComponent.K2_SetRelativeRotation` (`self.LeverMesh`) (`KismetMathLibrary.MakeRotator` _leverxrotation) false false))))

(fn `OnRep_WeaponSlotMachineWBP`)

(fn `UserConstructionScript`)