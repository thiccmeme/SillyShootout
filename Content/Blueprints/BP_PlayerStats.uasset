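; BP_PlayerStats tracks a player's health and death state.
; TakeDamage lowers CurrentHP to a floor of zero, sets IsDead, prints the HP for debugging and returns the death flag, skipping everything once dead.
; IncreaseHP heals up to MaxHP without checking or clearing IsDead, and GetHPPercentage returns current over max HP as a ratio.
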(fn `GetHPPercentage`
  (returns (HPPercent :type "Float (double-precision)"))
  (return (/ (`self.CurrentHP`) (`self.MaxHP`))))

(fn `IncreaseHP`
  (params (Amount :type Integer))
  (set `self.CurrentHP` (`KismetMathLibrary.FMin` (+ Amount (`self.CurrentHP`)) (`self.MaxHP`))))

(fn `TakeDamage`
  (params (Amount :type Integer))
  (returns (IsDead :type Boolean))
  (if (not (`self.IsDead`))
    (set `self.CurrentHP` (`KismetMathLibrary.FMax` (- (`self.CurrentHP`) Amount)))
    (set `self.IsDead` (<= (`self.CurrentHP`) 0))
    (`KismetSystemLibrary.PrintString` (`KismetStringLibrary.Concat_StrStr` "HP : " (`KismetStringLibrary.Conv_DoubleToString` (`self.CurrentHP`))))
    (return (`self.IsDead`))))