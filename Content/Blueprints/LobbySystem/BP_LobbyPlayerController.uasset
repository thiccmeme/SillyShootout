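; BP_LobbyPlayerController is the lobby player controller that creates each player's lobby UI and passes their lobby info to the game mode.
; On BeginPlay, SetUp shows the cursor and adds WBP_LobbyUI for local controllers only.
; SetPlayerNameOnServer stores the name in the controller's lobby info struct and has BP_LobbyGM update it.
; TryAgainUpdateLobbyInfo repeats that game mode update after a short delay.
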(event `self.ReceiveBeginPlay`
  (`self.SetUp`))

(event `TryAgainUpdateLobbyInfo`
  (`KismetSystemLibrary.Delay` 0.1)
  (bind _asbp_lobby_gm (cast `/Game/Blueprints/LobbySystem/BP_LobbyGM` (`GameplayStatics.GetGameMode`)))
  (`/Game/Blueprints/LobbySystem/BP_LobbyGM.UpdatePlayerLobbyInfo` _asbp_lobby_gm self))

(event `SetPlayerNameOnServer`
  (params (PlayerName :type Text))
  (setmembers `/Game/Blueprints/LobbySystem/S_PlayerLobbyInfo` :`StructRef` (`self.PlayerLobbyInfoPlayerController`) :`PlayerName` PlayerName)
  (bind _asbp_lobby_gm (cast `/Game/Blueprints/LobbySystem/BP_LobbyGM` (`GameplayStatics.GetGameMode`)))
  (`/Game/Blueprints/LobbySystem/BP_LobbyGM.UpdatePlayerLobbyInfo` _asbp_lobby_gm self))

(fn `SetUp`
  (if (`self.IsLocalPlayerController`)
    (set `self.bShowMouseCursor` true)
    (`WidgetBlueprintLibrary.SetInputMode_GameAndUIEx` self null "DoNotLock" false)
    (bind _returnvalue (`|CreateWidget` "/Game/Blueprints/LobbySystem/WBP_LobbyUI.WBP_LobbyUI_C"))
    (bind _output_get (set `self.LobbyUIRef` _returnvalue))
    (`UserWidget.AddToViewport` _output_get 0)))

(fn `UserConstructionScript`)