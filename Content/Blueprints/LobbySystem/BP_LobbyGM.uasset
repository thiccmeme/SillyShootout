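; Lobby game mode that assigns connected players to character platforms and relays their lobby info.
; On BeginPlay it collects platforms in order by index tag, and login or logout waits via a polling delay macro until that finishes.
; Each update spawns characters on free platforms for new controllers and clears departed ones.
; Info requests push name and ready state to the player's character, or ask the controller to retry if no platform matches.
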(event `self.ReceiveBeginPlay`
  (`self.SetUpPlatforms`))

(event `self.K2_PostLogin`
  (params (NewPlayer :type "PlayerController Object Reference"))
  (`KismetArrayLibrary.Array_Add` (`self.PlayerControllers`) NewPlayer)
  (`self.IfPlatformsSetUpDone`
    (:`true`
      (`self.UpdatePlayersOnPlatforms`))))

(event `self.K2_OnLogout`
  (params (ExitingController :type "Controller Object Reference"))
  (bind _asplayer_controller (cast `PlayerController` ExitingController))
  (`KismetArrayLibrary.Array_RemoveItem` (`self.PlayerControllers`) _asplayer_controller)
  (`self.IfPlatformsSetUpDone`
    (:`true`
      (`self.UpdatePlayersOnPlatforms`))))

(fn `SetUpPlatforms`
  ; Set players in the platforms
  (bind _outactors (`GameplayStatics.GetAllActorsOfClass` "/Game/Blueprints/LobbySystem/BP_LobbyPlayerPlatform.BP_LobbyPlayerPlatform_C"))
  (for _index (range (+ (`KismetArrayLibrary.Array_LastIndex` _outactors) 1))
    (bind _outactors_2 (`GameplayStatics.GetAllActorsOfClassWithTag` "/Game/Blueprints/LobbySystem/BP_LobbyPlayerPlatform.BP_LobbyPlayerPlatform_C" (`KismetStringLibrary.Conv_StringToName` (`KismetStringLibrary.Conv_IntToString` _index))))
    (`KismetArrayLibrary.Array_Add` (`self.PlayerPlatforms`) (`|GetArrayItem` _outactors_2)))
  (set `self.bPlatformsSetUpDone` true))

(fn `UpdatePlayerLobbyInfo`
  (params (RequestPlayerController :type "PlayerController Object Reference"))
  (bind _requestplayercontroller (`local.RequestPlayerController`))
  (for _array_element (`self.PlayerPlatforms`)
    (if (== (`/Game/Blueprints/LobbySystem/BP_LobbyPlayerPlatform.PlayerController` _array_element) RequestPlayerController)
      (bind _asbp_first_person_character (cast `/Game/FirstPerson/Blueprints/BP_FirstPersonCharacter` (`/Game/Blueprints/LobbySystem/BP_LobbyPlayerPlatform.CurrentCharacter` _array_element)))
      (`/Game/FirstPerson/Blueprints/BP_FirstPersonCharacter.UpdatePlayerLobbyInfo` _asbp_first_person_character (make `/Game/Blueprints/LobbySystem/S_PlayerLobbyInfo` _requestplayercontroller (`KismetTextLibrary.Conv_StringToText` (`AdvancedSessionsLibrary.GetPlayerName` _requestplayercontroller)) (`.bPlayerIsReady_8_183945D341C5BE4123917D80535B695A` (break `/Game/Blueprints/LobbySystem/S_PlayerLobbyInfo` (`/Game/Blueprints/LobbySystem/BP_LobbyPlayerController.PlayerLobbyInfoPlayerController` (cast `/Game/Blueprints/LobbySystem/BP_LobbyPlayerController` (`local.RequestPlayerController`) :!pure true)))) (`Controller.PlayerState` _requestplayercontroller)))
      (return)))
  (`/Game/Blueprints/LobbySystem/BP_LobbyPlayerController.TryAgainUpdateLobbyInfo` (cast `/Game/Blueprints/LobbySystem/BP_LobbyPlayerController` (`local.RequestPlayerController`) :!pure true)))

(fn `UpdatePlayersOnPlatforms`
  (locals (bPlayerControllerAlreadyAdded :type Boolean))
  ; Check if Player Controller is already in the platform
  (for _array_element (`self.PlayerControllers`)
    (set `local.bPlayerControllerAlreadyAdded` false)
    (for _array_element_2 (`self.PlayerPlatforms`)
      (if (== (`/Game/Blueprints/LobbySystem/BP_LobbyPlayerPlatform.PlayerController` _array_element_2) _array_element)
        (set `local.bPlayerControllerAlreadyAdded` true)
        (break)))
    ; Add Player Controller to platforms if needed
    (if (not (`local.bPlayerControllerAlreadyAdded`))
      (for _array_element_3 (`self.PlayerPlatforms`)
        (`/Engine/EditorBlueprintResources/StandardMacros.IsValid` (`/Game/Blueprints/LobbySystem/BP_LobbyPlayerPlatform.PlayerController` _array_element_3)
          (:`Is Not Valid`
            (`/Game/Blueprints/LobbySystem/BP_LobbyPlayerPlatform.SpawnCharacter` _array_element_3 _array_element)
            (break))))))
  ; Remove disconnected players from the platforms
  (for _array_element_4 (`self.PlayerPlatforms`)
    (if (not (`KismetArrayLibrary.Array_Contains` (`self.PlayerControllers`) (`/Game/Blueprints/LobbySystem/BP_LobbyPlayerPlatform.PlayerController` _array_element_4)))
      (`/Game/Blueprints/LobbySystem/BP_LobbyPlayerPlatform.ClearCharacter` _array_element_4))))

(fn `UserConstructionScript`)