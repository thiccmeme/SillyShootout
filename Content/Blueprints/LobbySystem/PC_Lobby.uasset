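; Player controller for the lobby, holding this player's lobby info (name and ready state) and passing it to GM_Lobby.
; On BeginPlay, the local controller shows the cursor, creates the lobby UI and submits the player's name through SetPlayerNameOnServer.
; Name changes and ready toggles edit the info struct, then call UpdatePlayerLobbyInfo on the game mode.
; TryAgainUpdateLobbyInfo repeats that update after a short delay.
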(event `self.ReceiveBeginPlay`
  (`self.SetUp`))

(event `TryAgainUpdateLobbyInfo`
  (`KismetSystemLibrary.Delay` 0.1)
  (bind _asbp_lobby_gm (cast `/Game/Blueprints/LobbySystem/GM_Lobby` (`GameplayStatics.GetGameMode`)))
  (`/Game/Blueprints/LobbySystem/GM_Lobby.UpdatePlayerLobbyInfo` _asbp_lobby_gm self))

(event `SetPlayerNameOnServer`
  (params (PlayerName :type Text))
  (setmembers `/Game/Blueprints/LobbySystem/S_PlayerLobbyInfo` :`StructRef` (`self.PlayerLobbyInfoPlayerController`) :`PlayerName` PlayerName)
  (bind _asbp_lobby_gm (cast `/Game/Blueprints/LobbySystem/GM_Lobby` (`GameplayStatics.GetGameMode`)))
  (`/Game/Blueprints/LobbySystem/GM_Lobby.UpdatePlayerLobbyInfo` _asbp_lobby_gm self))

(event `ToggleReadyStatusOnServer`
  (bind _returnvalue (`GameplayStatics.GetGameMode`))
  (bind _playerlobbyinfoplayercontroller (`self.PlayerLobbyInfoPlayerController`))
  (setmembers `/Game/Blueprints/LobbySystem/S_PlayerLobbyInfo` :`StructRef` _playerlobbyinfoplayercontroller :`bPlayerIsReady` (not (`.bPlayerIsReady_8_183945D341C5BE4123917D80535B695A` (break `/Game/Blueprints/LobbySystem/S_PlayerLobbyInfo` _playerlobbyinfoplayercontroller))))
  (bind _asbp_lobby_gm (cast `/Game/Blueprints/LobbySystem/GM_Lobby` _returnvalue)
    (:`then`
      (`/Game/Blueprints/LobbySystem/GM_Lobby.UpdatePlayerLobbyInfo` _asbp_lobby_gm self))
    (:`CastFailed`
      (`KismetSystemLibrary.PrintString` (`KismetSystemLibrary.GetObjectName` _returnvalue))
      (`KismetSystemLibrary.PrintString` "Failed"))))

(fn `SetUp`
  (if (`self.IsLocalPlayerController`)
    (set `self.bShowMouseCursor` true)
    (`WidgetBlueprintLibrary.SetInputMode_GameAndUIEx` self null "DoNotLock" false)
    (bind _returnvalue (`|CreateWidget` "/Game/Blueprints/LobbySystem/WBP_LobbyUI.WBP_LobbyUI_C"))
    (bind _output_get (set `self.LobbyUIRef` _returnvalue))
    (`UserWidget.AddToViewport` _output_get 0)
    (`self.SetPlayerNameOnServer` (`KismetTextLibrary.Conv_StringToText` (`AdvancedSessionsLibrary.GetPlayerName` null)))))

(fn `UserConstructionScript`)