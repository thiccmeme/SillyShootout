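; Lobby platform Blueprint that displays a character for an assigned player controller.
; SpawnCharacter stores the controller, destroys any existing character and spawns a BP_FirstPersonCharacter at the PlayerTransform component's world transform, without possessing it.
; ClearCharacter releases the controller reference and destroys the current character, emptying the platform.
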(event `SpawnCharacter`
  (params (PlayerController :type "PlayerController Object Reference"))
  (bind _currentcharacter (`self.CurrentCharacter`))
  ; Spawn character on the platforms
  (set `self.PlayerController` PlayerController)
  (`/Engine/EditorBlueprintResources/StandardMacros.IsValid` _currentcharacter
    (:`Is Valid`
      (`self.K2_DestroyActor` _currentcharacter))
    (:`Is Not Valid`
      _))
  (bind _returnvalue (`|SpawnActorFromClass` "/Game/FirstPerson/Blueprints/BP_FirstPersonCharacter.BP_FirstPersonCharacter_C" (`SceneComponent.K2_GetComponentToWorld` (`self.PlayerTransform`)) "Undefined" "MultiplyWithRoot" null null))
  (set `self.CurrentCharacter` _returnvalue))

(event `ClearCharacter`
  (bind _currentcharacter (`self.CurrentCharacter`))
  ; Remove character from the platforms
  (set `self.PlayerController` null)
  (`/Engine/EditorBlueprintResources/StandardMacros.IsValid` _currentcharacter
    (:`Is Valid`
      (`self.K2_DestroyActor` _currentcharacter)
      (set `self.CurrentCharacter` null))))

(fn `UserConstructionScript`)